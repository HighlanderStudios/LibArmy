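; Day/night cycle Blueprint that animates sun, sky, fog and artificial lighting over a looping 24-hour clock.
; Tick advances Time by a time scale and uses it to scrub SunTimeline, whose curves set sun pitch, intensity and artificial light level.
; These drive the main light, skylight, skysphere and DynamicLights, while height fog density and scattering rise steeply as sunlight fades.
; The light-color helper graphs contain only unused nodes.
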(event EventTick
  (params (DeltaSeconds :type Float%20%28single-precision%29))
  (bind _heightfog (Variables|Default|GetHeightFog))
  (bind _output_get (Variables|Default|SetTime (Math|Float|%(Float) (+ (/ DeltaSeconds (Variables|Default|GetTimeScale)) (Variables|Default|GetTime)) 24.0)))
  (bind (_direction _sunpitch _intensity _artificial_lights) (Timeline|SunTimeline SetNewTime)
    (:Update
      (Variables|Default|SetCurrentLightIntensity _intensity)
      (Transformation|SetActorRotation (Variables|Default|GetMainLight) (Math|Rotator|MakeRotator 0.0 _sunpitch 1.8e+02))
      (Rendering|Components|Light|SetIntensity (Variables|Default|GetMainLight) (* (Variables|Default|GetCurrentLightIntensity) 3.14))
      (Rendering|Components|Light|SetIntensity (Variables|/Script/Engine.SkyLight|GetLightComponent (Variables|Default|GetSkylight)) (+ (* (Variables|Default|GetCurrentLightIntensity) (Variables|Default|GetSkylightMultiplier)) (Variables|Default|GetSkylightBase)))
      (Default|UpdateSunDirection (Variables|Default|GetSkysphere))
      (Class|ExponentialHeightFogComponent|SetVolumetricFogScatteringDistribution (Variables|/Script/Engine.ExponentialHeightFog|GetComponent _heightfog) (* (Math|Float|Power (- 1.0 (Variables|Default|GetCurrentLightIntensity)) 6.0) 0.5))
      (Class|ExponentialHeightFogComponent|SetFogDensity (Variables|/Script/Engine.ExponentialHeightFog|GetComponent _heightfog) (* (Math|Float|Power (- 1.0 (Variables|Default|GetCurrentLightIntensity)) 6.0) 0.5))
      (for _array_element (Variables|Default|GetDynamicLights)
        (Rendering|Components|Light|SetIntensity (Variables|/Script/Engine.Light|GetLightComponent _array_element) (* _artificial_lights 5e+04))))))

(fn ConstructionScript)